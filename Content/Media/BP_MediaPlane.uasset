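; BP_MediaPlane is a media plane actor with on-screen video playback controls.
; On BeginPlay it creates a VideoControll widget, adds it to the viewport and binds three of its button click events.
; The clicks respectively call OpenMedia, rescale the Plane component to PlaneSize before playing the MediaPlayer, and pause the MediaPlayer.
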(event Custom|OnClicked_Event_0
  (Class|VideoPlane|OpenMedia))

(event Custom|OnClicked_Event_1
  (Transformation|SetWorldScale3D (Variables|Default|GetPlane) (Variables|Default|GetPlaneSize))
  (Media|MediaPlayer|Play (Variables|Default|GetMediaPlayer) :!class /Script/MediaAssets.MediaPlayer))

(event Custom|OnClicked_Event_2
  (Sequencer|Player|Pause (Variables|Default|GetMediaPlayer)))

(event EventBeginPlay
  (bind _returnvalue (UserInterface|CreateWidget "/Game/Widgets/VideoControll.VideoControll_C"))
  (bind _output_get (Variables|Default|SetControll _returnvalue))
  (UserInterface|Viewport|AddtoViewport _output_get 0)
  (EventDispatchers|AssignOnClicked (Variables|/Game/Widgets/VideoControll.VideoControll_C|GetButton_0 (Variables|Default|GetControll)) (delegate Custom|OnClicked_Event_0))
  (EventDispatchers|AssignOnClicked (Variables|/Game/Widgets/VideoControll.VideoControll_C|GetButton (Variables|Default|GetControll)) (delegate Custom|OnClicked_Event_1))
  (EventDispatchers|AssignOnClicked (Variables|/Game/Widgets/VideoControll.VideoControll_C|GetButton_1 (Variables|Default|GetControll)) (delegate Custom|OnClicked_Event_2)))

(event Collision|EventActorBeginOverlap
  (params (OtherActor :type Actor%20Object%20Reference)))

(event EventTick
  (params (DeltaSeconds :type Float%20%28single-precision%29)))

(fn ConstructionScript)